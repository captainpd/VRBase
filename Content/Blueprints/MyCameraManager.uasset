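; A player camera manager for a VR pawn that computes a camera view from the headset or a motion controller, picked by CamTarget.
; BeginPlay caches those components, and GetCameraStats returns the chosen one's transform with a fixed FOV, though Left Hand reuses Target instead of HandLeft.
; BlueprintUpdateCamera copies that view when the target is unchanged, otherwise lerps toward it without updating LastCamTarget.
; Both branches return false.
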(event EventBeginPlay
  (bind _asvr_pawn (Utilities|Casting|CastToVR_Pawn (Game|Player|GetPlayerPawn 0)))
  (Variables|Default|SetHMD (Variables|/Game/00_VRBase/VR/VR_Pawn.VR_Pawn_C|GetHMDInfo _asvr_pawn))
  (Variables|Default|SetHand_Left (Variables|/Game/00_VRBase/VR/VR_Pawn.VR_Pawn_C|GetMotionController_Left _asvr_pawn))
  (Variables|Default|SetHand_Right (Variables|/Game/00_VRBase/VR/VR_Pawn.VR_Pawn_C|GetMotionController_Right _asvr_pawn)))

(event EventTick
  (params (DeltaSeconds :type Float%20%28single-precision%29)))

(fn ConstructionScript)

(fn BlueprintUpdateCamera
  (params (CameraTarget :type Actor%20Object%20Reference))
  (bind _camtarget (Variables|Default|GetCamTarget))
  (if (Utilities|Enum|Equal(Enum) (LocalVariables|GetLastCamTarget) (Variables|Default|GetCamTarget))
    (Variables|Default|SetCamStat "NewEnumerator0")
    (bind (__location __rotation __fov) (CallFunction|GetCameraStats _camtarget))
    (LocalVariables|SetLastCamTarget _camtarget)
    (return __location __rotation __fov false)
    (else
      (Variables|Default|SetCamStat "NewEnumerator1")
      (bind (__location_2 __rotation_2 __fov_2) (CallFunction|GetCameraStats (Variables|Default|GetCamTarget)))
      (return (Math|Vector|Lerp(Vector) (Transformation|GetActorLocation CameraTarget) __location_2 0.1) (Math|Rotator|Lerp(Rotator) (Transformation|GetActorRotation CameraTarget) __rotation_2 0.1) (Math|Float|Lerp (Variables|/Script/Engine.CameraComponent|GetFieldOfView (Variables|/Script/Engine.CameraActor|GetCameraComponent (.AsCamera%20Actor (Utilities|Casting|CastToCameraActor CameraTarget)))) __fov_2 0.1) false))))

(fn GetCameraStats
  (params (CamTarget :type CamTarget%20Enum :default "NewEnumerator0"))
  (switch Utilities|FlowControl|Switch|SwitchonCamTarget CamTarget
    (:NewEnumerator0
      (LocalVariables|Set_Target (Variables|Default|GetHMD)))
    (:NewEnumerator1
      (LocalVariables|Set_Target (LocalVariables|Get_Target)))
    (:NewEnumerator2
      (LocalVariables|Set_Target (Variables|Default|GetHand_Right))))
  (LocalVariables|SetLocation (Transformation|GetWorldLocation (LocalVariables|Get_Target)))
  (LocalVariables|SetRotation (Transformation|GetWorldRotation (LocalVariables|Get_Target)))
  (LocalVariables|SetFielfOfView 9e+01)
  (return (LocalVariables|GetLocation) (LocalVariables|GetRotation) (LocalVariables|GetFielfOfView)))